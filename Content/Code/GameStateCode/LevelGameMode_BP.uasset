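; Level game mode that brackets each level with scoring and timing.
; On BeginPlay it caches the BadBoyGameInstance, starts scoring with the current food wad's total restoration truncated to an integer, then starts the instance's level timer.
; EndLevel recomputes that restoration total to end scoring, then pauses the timer.
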(event Custom|EndLevel
  (Utilities|FlowControl|Sequence
    (:then_0
      (bind _totalrestoration (CallFunction|FoodWadTotalRestoration (Variables|/Game/Code/GameStateCode/BadBoyGameInstance.BadBoyGameInstance_C|GetCurrentFoodWad (Variables|Default|GetBad%20Boy%20Game%20Instance))))
      (Class|LevelGameMode|EndLevelScoring (Math|Float|Truncate _totalrestoration)))
    (:then_1
      (Default|PauseLevelTimer (Variables|Default|GetBad%20Boy%20Game%20Instance)))))

(event EventBeginPlay
  (bind _asbad_boy_game_instance (Utilities|Casting|CastToBadBoyGameInstance (Game|GetGameInstance)))
  (bind _output_get (Variables|Default|SetBad%20Boy%20Game%20Instance _asbad_boy_game_instance))
  (Utilities|FlowControl|Sequence
    (:then_0
      (bind _totalrestoration (CallFunction|FoodWadTotalRestoration (Variables|/Game/Code/GameStateCode/BadBoyGameInstance.BadBoyGameInstance_C|GetCurrentFoodWad _output_get)))
      (Class|LevelGameMode|StartLevelScoring (Math|Float|Truncate _totalrestoration)))
    (:then_1
      (Default|StartLevelTimer _output_get))))

(event EventTick
  (params (DeltaSeconds :type Float%20%28single-precision%29)))

(fn ConstructionScript)